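; Pressable red button that fills a progress bar, which drains on a looping timer and is shown through a dynamic material on a cube.
; An overlapping component pushes the button down on Tick, and each full press plays a sound, adds progress and resumes the timer.
; The button eases back with VInterpTo when released.
; Reaching full progress plays a sound once, then after a delay fires every BP_Display actor.
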(event `self.ReceiveBeginPlay`
  (set `self.Init_Location` (`SceneComponent.RelativeLocation` (`self.Red_Button`)))
  ;[1 1 1] ProgressBar Material
  (bind _returnvalue (`PrimitiveComponent.CreateDynamicMaterialInstance` (`self.Cube`) 0 "/Game/TestTask/Materials/M_ProgressBar.M_ProgressBar" "None"))
  (set `self.DynamicMaterial` _returnvalue)
  (`KismetSystemLibrary.K2_SetTimer` self "LoweringProgress" (`self.TimerTick`) true))

(event `self.ReceiveTick`
  (params (DeltaSeconds :type "Float (single-precision)"))
  (bind _red_button (`self.Red_Button`))
  (bind (_returnvalue_x _returnvalue_y _returnvalue_z) (`KismetMathLibrary.BreakVector` (- (`KismetMathLibrary.InverseTransformDirection` (`SceneComponent.K2_GetComponentToWorld` _red_button) (`self.Start Location`)) (`KismetMathLibrary.InverseTransformDirection` (`SceneComponent.K2_GetComponentToWorld` _red_button) (`SceneComponent.K2_GetComponentLocation` (`self.Overlap`))))))
  (bind _returnvalue (`KismetMathLibrary.FClamp` _returnvalue_z 0.0 (`self.MaxButtonPress`)))
  ;[1 1 1] Smooth Button Press
  (`/Engine/EditorBlueprintResources/StandardMacros.IsValid` (`self.Overlap`)
    (:`Is Valid`
      (set `self.ButtonPressAmount` _returnvalue)
      (`SceneComponent.K2_SetRelativeLocation` (`self.Red_Button`) (- (`self.Init_Location`) (`KismetMathLibrary.MakeVector` 0.0 0.0 _returnvalue)) false false)
      (if (>= (`self.ButtonPressAmount`) (`self.MaxButtonPress`))
        (`/Engine/EditorBlueprintResources/StandardMacros.DoOnce` false :!label _label
          (:`Completed`
            (`GameplayStatics.PlaySound2D` "/Game/TestTask/Audio/Button/key.key" 1.0 1.0 0.0 null null)
            (`KismetSystemLibrary.K2_UnPauseTimer` self "LoweringProgress")
            (set `self.Progress` (+ (`self.Progress`) (`self.ProgressAddButtonAmount`)))))
        (else
          (goto _label :!via `Reset`))))
    (:`Is Not Valid`
      (`SceneComponent.K2_SetRelativeLocation` (`self.Red_Button`) (`KismetMathLibrary.VInterpTo` (`SceneComponent.RelativeLocation` (`self.Red_Button`)) (`self.Init_Location`) DeltaSeconds 8.0) false false))))

(event `self.Red_Button.OnComponentBeginOverlap`
  (params (OverlappedComponent :type "PrimitiveComponent Object Reference") (OtherActor :type "Actor Object Reference") (OtherComp :type "PrimitiveComponent Object Reference") (OtherBodyIndex :type Integer) (bFromSweep :type Boolean) (SweepResult :type "HitResult Structure (by ref)"))
  ;[1 1 1] Smooth Button Press
  (`/Engine/EditorBlueprintResources/StandardMacros.IsValid` (`self.Overlap`)
    (:`Is Not Valid`
      (bind _output_get (set `self.Overlap` OtherComp))
      (set `self.Start Location` (`SceneComponent.K2_GetComponentLocation` _output_get)))))

(event `self.Red_Button.OnComponentEndOverlap`
  (params (OverlappedComponent :type "PrimitiveComponent Object Reference") (OtherActor :type "Actor Object Reference") (OtherComp :type "PrimitiveComponent Object Reference") (OtherBodyIndex :type Integer))
  ;[1 1 1] Smooth Button Press
  (if (== OtherComp (`self.Overlap`))
    (set `self.Overlap` null)))

(event `100Progress`
  ;[1 1 1] Send Event to lift display
  (`/Engine/EditorBlueprintResources/StandardMacros.DoOnce` false
    (:`Completed`
      (`GameplayStatics.PlaySound2D` "/Game/TestTask/Audio/Siren/ezz.ezz" 1.0 1.0 0.0 null null)
      (`KismetSystemLibrary.Delay` 1.42)
      (bind _outactors (`GameplayStatics.GetAllActorsOfClass` "/Game/TestTask/BP_Display.BP_Display_C"))
      (for _array_element _outactors
        (`/Game/TestTask/BP_Display.FireDisplay` _array_element)))))

(fn `LoweringProgress`
  (bind _progress (`self.Progress`))
  (`MaterialInstanceDynamic.SetScalarParameterValue` (`self.DynamicMaterial`) "ProgressParam" (`self.Progress`))
  (if (or (>= _progress 1.0) (< _progress 0.0))
    (`KismetSystemLibrary.K2_PauseTimer` self "LoweringProgress")
    (if (>= (`self.Progress`) 1.0)
      (`self.100Progress`))
    (else
      (set `self.Progress` (- (`self.Progress`) (`self.LoweringProgressByTick`))))))

(fn `UserConstructionScript`)