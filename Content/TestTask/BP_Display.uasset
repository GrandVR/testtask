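; BP_Display is a display screen actor that rises and plays a teaser movie when its FireDisplay event is called.
; FireDisplay plays a loud sound at the Plane, then runs a timeline as a tick driver, easing the Plane's world height toward a fixed target with FInterpTo.
; When the timeline finishes, it activates the media sound component and opens the Priest vs. Poltergeist teaser on the media player.
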(event `FireDisplay`
  (bind (_returnvalue_x _returnvalue_y _returnvalue_z) (`KismetMathLibrary.BreakVector` (`SceneComponent.K2_GetComponentLocation` (`self.Plane`))))
  (`GameplayStatics.SpawnSoundAtLocation` "/Game/TestTask/Audio/Target/TARGET.TARGET" (`SceneComponent.K2_GetComponentLocation` (`self.Plane`)) (struct) 5.0 1.0 0.0 null null)
  ;[1 1 1] Smooth Lift Display
  (`Timeline|Timeline_0` :!via `PlayFromStart`
    (:`Update`
      (`SceneComponent.K2_SetWorldLocation` (`self.Plane`) (`KismetMathLibrary.MakeVector` _returnvalue_x _returnvalue_y (`KismetMathLibrary.FInterpTo` _returnvalue_z 300.0 (`GameplayStatics.GetWorldDeltaSeconds`) 3.0)) false false))
    (:`Finished`
      ;[1 1 1] Start Movie
      (`ActorComponent.SetActive` (`self.MediaSound`) true false)
      (`MediaPlayer.OpenSource` (`self.MediaPlayer`) "/Game/TestTask/Movies/Priest_vs__Poltergeist_Teaser.Priest_vs__Poltergeist_Teaser"))))

(fn `UserConstructionScript`)